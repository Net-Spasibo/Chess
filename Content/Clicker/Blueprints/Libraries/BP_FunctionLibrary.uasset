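; Blueprint function library for the clicker game that looks up enemy, level, item, item cost and ascension data in data tables.
; Each function converts its input to a row name, using Replace on enemy and item names and stringifying numeric levels and counts.
; Item cost reads the row one above the amount bought, so it gives the next purchase's entry.
; Only the Row Found path returns a row.
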(fn FGetEnemyInfo
  (params (EnemyName :type String))
  (bind _returnvalue (Utilities|GetDataTableRow "/Game/Clicker/Blueprints/DataTables/DT_EnemyInfo.DT_EnemyInfo" (Utilities|String|StringToName (Utilities|String|Replace EnemyName " ")))
    (:then
      (return _returnvalue))))

(fn FGetLevelInfo
  (params (Level :type Integer))
  (bind _returnvalue (Utilities|GetDataTableRow "/Game/Clicker/Blueprints/DataTables/DT_LevelInfo.DT_LevelInfo" (Utilities|String|StringToName (Utilities|String|ToString(Integer) Level)))
    (:then
      (return _returnvalue))))

(fn FGetItemInfo
  (params (ItemName :type String))
  (bind _returnvalue (Utilities|GetDataTableRow "/Game/Clicker/Blueprints/DataTables/DT_ItemInfo.DT_ItemInfo" (Utilities|String|StringToName (Utilities|String|Replace ItemName " ")))
    (:then
      (return _returnvalue))))

(fn FGetItemCost
  (params (AmountOfItemsBought :type Integer))
  (bind _returnvalue (Utilities|GetDataTableRow "/Game/Clicker/Blueprints/DataTables/DT_ItemCost.DT_ItemCost" (Utilities|String|StringToName (Utilities|String|ToString(Integer) (+ AmountOfItemsBought 1))))
    (:then
      (return _returnvalue))))

(fn FGetAscensionDamageMultiplier
  (params (AscensionLevel :type Integer))
  (bind _returnvalue (Utilities|GetDataTableRow "/Game/Clicker/Blueprints/DataTables/DT_Ascension.DT_Ascension" (Utilities|String|StringToName (Utilities|String|ToString(Integer) AscensionLevel)))
    (:then
      (return _returnvalue))))