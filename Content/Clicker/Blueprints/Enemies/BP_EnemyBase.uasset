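; Base clickable flipbook enemy for a clicker game, with health bar and info widgets, driven by per-name enemy data.
; Clicks apply the player's cursor damage with floating text, sound and a hit animation, after which death triggers at zero health.
; AutoDamage kills trigger death directly, avoiding conflict with the click path.
; Death runs once, stopping the round timer, awarding coins, then unlocking and setting the level through the GameMode before destruction.
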(event OnClicked(CapsuleComponent)
  (params (TouchedComponent :type Primitive%20Component%20Object%20Reference) (ButtonPressed :type Key%20Structure :default "None"))
  ;[0.1412 0.2667 0.8431 0.3608] The mouse clicking event - Applies damage to enemy
  (if (not (Variables|EnemyProperties|GetbIsDead))
    (Game|Damage|ApplyDamage self (Variables|/Game/Clicker/Blueprints/Player/BP_Player.BP_Player_C|GetCursorDamage (Variables|References|GetPlayerPawn)) 0 0)
    (Default|SpawnFloatingText (Variables|References|GetPlayerController) (Utilities|String|ToString(Float) (Variables|/Game/Clicker/Blueprints/Player/BP_Player.BP_Player_C|GetCursorDamage (Variables|References|GetPlayerPawn))) (Transformation|GetActorLocation))
    (CallFunction|HitEffect)
    (Audio|PlaySound2D (Variables|SFX|GetPunchSFX) 1.0 1.0 0.0 0 0)))

(event Custom|UpdateHealth
  (params (CurrentHealth :type Float%20%28double-precision%29))
  ;[0.1412 0.2667 0.8431 0.3608] Updates the enemy health
  (Variables|EnemyProperties|SetCurrentHealth CurrentHealth)
  (bind _aswb_health_bar (Utilities|Casting|CastToWB_HealthBar (UserInterface|GetUserWidgetObject (Variables|Default|GetHealthBarWidget))))
  (Default|UpdateHealthUI _aswb_health_bar (Variables|EnemyProperties|GetCurrentHealth) (Utilities|Struct|BreakST_EnemyInfo (CallFunction|FGetEnemyInfo (Variables|EnemyProperties|GetName)))))

(event Custom|HitEffect
  (bind _name (Variables|EnemyProperties|GetName))
  (bind _enemyinfo (CallFunction|FGetEnemyInfo _name))
  (bind (_idleanim _hitanim) (Utilities|Struct|BreakST_EnemyInfo _enemyinfo))
  ;[0.1412 0.2667 0.8431 0.3608] Enemy mouse hit VFX
  (Sprite|SetFlipbook (Variables|Default|GetSprite) _hitanim)
  (Utilities|FlowControl|Delay (Class|PaperFlipbookComponent|GetFlipbookLength (Variables|Default|GetSprite)))
  (if (Variables|EnemyProperties|GetbIsDead)
    (CallFunction|Death)
    (else
      (Sprite|SetFlipbook (Variables|Default|GetSprite) _idleanim))))

(event Custom|Death
  (bind _name (Variables|EnemyProperties|GetName))
  (bind _gamemode (Variables|References|GetGameMode))
  (bind _enemyinfo (CallFunction|FGetEnemyInfo _name))
  (bind (_deathanim _deathsfx) (Utilities|Struct|BreakST_EnemyInfo _enemyinfo))
  ;[0.1412 0.2667 0.8431 0.3608] Enemy Death logic
  (Utilities|FlowControl|DoOnce false
    (:Completed
      (Utilities|Time|ClearandInvalidateTimerbyHandle (Variables|/Game/Clicker/Blueprints/GM_Clicker.GM_Clicker_C|GetRoundTimerHandle (Variables|References|GetGameMode)))
      (Audio|PlaySound2D _deathsfx 1.0 1.0 0.0 0 0)
      (Sprite|SetFlipbook (Variables|Default|GetSprite) _deathanim)
      (Components|Timeline|SetLooping (Variables|Default|GetSprite) false)
      (Default|UpdateAmountOfCoins (Variables|References|GetPlayerPawn) (Utilities|Struct|BreakST_EnemyInfo (CallFunction|FGetEnemyInfo (Variables|EnemyProperties|GetName))) true)
      (Default|FUpdateShopItemCardBuyTextColor (Variables|References|GetPlayerController))
      (Utilities|FlowControl|Delay (Class|PaperFlipbookComponent|GetFlipbookLength (Variables|Default|GetSprite)))
      (Default|UnlockLevel _gamemode)
      (Default|SetCurrentLevel _gamemode (Variables|/Game/Clicker/Blueprints/GM_Clicker.GM_Clicker_C|GetCurrentLevel _gamemode))
      (Actor|DestroyActor))))

(event Custom|RestoreHealth
  ;[0.1412 0.2667 0.8431 0.3608] Restores the enemy health
  (CallFunction|UpdateHealth (.Health (Utilities|Struct|BreakST_EnemyInfo (CallFunction|FGetEnemyInfo (Variables|EnemyProperties|GetName))))))

(event EventBeginPlay
  ;[0.1412 0.2667 0.8431 0.3608] Begin Play - Defines variables and updates the Health and UI for the enemy.
  (bind _gamemode (Class|BPIGameMode|GetGameModeRef(Message) (Game|GetGameMode)))
  (Variables|References|SetGameMode _gamemode)
  (bind _playercontroller (Class|BPIPlayerController|GetPlayerControllerRef(Message) (Game|GetPlayerController 0)))
  (Variables|References|SetPlayerController _playercontroller)
  (bind _player (Class|BPIPlayer|GetPlayerRef(Message) (Game|GetPlayerCharacter 0)))
  (Variables|References|SetPlayerPawn _player)
  (bind _aswb_enemy_info (Utilities|Casting|CastToWB_EnemyInfo (UserInterface|GetUserWidgetObject (Variables|Default|GetEnemyInfoWidget))))
  (Default|UpdateEnemyInfoUI _aswb_enemy_info (Variables|EnemyProperties|GetName) (Variables|/Game/Clicker/Blueprints/GM_Clicker.GM_Clicker_C|GetCurrentLevel (Variables|References|GetGameMode))))

(event Game|Damage|EventAnyDamage
  (params (Damage :type Float%20%28single-precision%29) (DamageType :type Damage%20Type%20Object%20Reference) (InstigatedBy :type Controller%20Object%20Reference) (DamageCauser :type Actor%20Object%20Reference))
  (bind _currenthealth (Variables|EnemyProperties|GetCurrentHealth))
  (bind _currenthealth_2 (Variables|EnemyProperties|GetCurrentHealth))
  (bind _returnvalue (- _currenthealth_2 Damage))
  (bind _returnvalue_2 (Math|Float|Clamp(Float) _returnvalue 0.0 _currenthealth))
  ;[0.1412 0.2667 0.8431 0.3608] Enemy takes damage and updates the health.
  (if (> _returnvalue_2 0.0)
    _
    (else
      (Variables|EnemyProperties|SetbIsDead true)))
  (CallFunction|UpdateHealth _returnvalue_2)
  ;;[0.1412 0.2667 0.8431 0.3608] This is added to prevent the autodamage logic from playing the Death event when we click through the mouse.
  (if (and (Utilities|String|Contains (Utilities|GetDisplayName DamageType) "AutoDamage") (Variables|EnemyProperties|GetbIsDead))
    (CallFunction|Death)))

(fn ConstructionScript)