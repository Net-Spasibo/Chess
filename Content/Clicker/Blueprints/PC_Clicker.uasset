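; Player controller for the clicker game that owns the UI and spawns enemies, items, hit effects and floating text.
; On BeginPlay it caches the pawn, shows the main widget, sets a widget cursor, and fills a list with shop cards per DT_ItemInfo row plus a level card.
; Enum-driven show/hide lazily creates the main and ascension popup widgets.
; Shop buy buttons are colored and enabled by comparing item cost against the pawn's coins.
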(event Custom|InitializePlayer
  ;[0.1412 0.2667 0.8431 0.3608] Initialize Player
  (bind _returnvalue (UserInterface|CreateWidget "/Game/Clicker/UI/WB_ShopTooltip.WB_ShopTooltip_C"))
  (Variables|Widgets|SetWB_ShopTooltip _returnvalue)
  (bind _returnvalue_2 (UserInterface|CreateWidget "/Game/Clicker/UI/WB_MouseCursor.WB_MouseCursor_C"))
  (bind _output_get (Variables|Widgets|SetWB_MouseCursor _returnvalue_2))
  (Class|PlayerController|SetMouseCursorWidget "Default" _output_get))

(event Custom|ShowHideWidget
  (params (Widget :type E_GameWidgets%20Enum :default "NewEnumerator0") (Show :type Boolean))
  (if Show
    (CallFunction|FShowWidget Widget)
    (else
      (CallFunction|FHideWidget Widget))))

(event Custom|SpawnItem
  (params (Item :type Actor%20Class%20Reference) (SpawnLocation :type Vector))
  (Game|SpawnActorfromClass Item (Math|Transform|MakeTransform SpawnLocation) "AlwaysSpawn" "MultiplyWithRoot" 0 0))

(event Custom|SpawnEnemy
  (params (Enemy :type Actor%20Class%20Reference) (SpawnTransform :type Transform))
  (bind _returnvalue (Game|SpawnActorfromClass Enemy SpawnTransform "AdjustIfPossibleButAlwaysSpawn" "MultiplyWithRoot" 0 0))
  (bind _enemy (Class|BPIEnemyBase|GetEnemyRef(Message) _returnvalue))
  (Variables|Default|SetSpawnedEnemy _enemy))

(event Custom|SpawnHitEffect
  (Game|SpawnActorfromClass "/Game/Clicker/Blueprints/BP_HitEffect.BP_HitEffect_C" (Math|Conversions|ToTransform(Vector) (- (.WorldLocation (Game|Player|ConvertMouseLocationToWorldSpace)) "0.000000,1.000000,0.000000")) "AlwaysSpawn" "MultiplyWithRoot" 0 0))

(event Custom|SpawnFloatingText
  (params (Text :type String) (SpawnLocation :type Vector))
  (bind (_x _y _z) (Math|Vector|BreakVector SpawnLocation))
  (Game|SpawnActorfromClass "/Game/Clicker/Blueprints/BP_FloatingText.BP_FloatingText_C" (Math|Transform|MakeTransform (Math|Vector|MakeVector _x 1.0 (+ _z 2e+01))) "AlwaysSpawn" "MultiplyWithRoot" 0 Text 0)
  (CallFunction|SpawnHitEffect))

(event Custom|CreateShopItemCards
  (Utilities|Array|Clear (Variables|Default|GetShopItemCards))
  (bind _outrownames (DataTable|GetDataTableRowNames "/Game/Clicker/Blueprints/DataTables/DT_ItemInfo.DT_ItemInfo"))
  (for _array_element _outrownames
    (bind _returnvalue (UserInterface|CreateWidget "/Game/Clicker/UI/WB_ShopItemCard.WB_ShopItemCard_C"))
    (Utilities|Array|Add (Variables|Default|GetShopItemCards) _returnvalue))
  (CallFunction|DisplayShopItemCards)
  (CallFunction|FUpdateShopItemCardBuyTextColor))

(event Custom|DisplayShopItemCards
  (Widget|Panel|ClearChildren (Variables|/Game/Clicker/UI/WB_Main.WB_Main_C|GetVB_ItemList (Variables|Widgets|GetWB_Main)))
  (for _array_element (Variables|Default|GetShopItemCards)
    (Class|VerticalBox|AddChildtoVerticalBox (Variables|/Game/Clicker/UI/WB_Main.WB_Main_C|GetVB_ItemList (Variables|Widgets|GetWB_Main)) _array_element)))

(event Custom|AddLevelButtonUI
  (params (Level :type Integer))
  (bind _returnvalue (UserInterface|CreateWidget "/Game/Clicker/UI/WB_LevelCard.WB_LevelCard_C" 0 Level))
  (Class|VerticalBox|AddChildtoVerticalBox (Variables|/Game/Clicker/UI/WB_Main.WB_Main_C|GetVB_ItemList (Variables|Widgets|GetWB_Main)) _returnvalue))

(event EventBeginPlay
  ;[0.1412 0.2667 0.8431 0.3608] Begin Play
  (bind _player (Class|BPIPlayer|GetPlayerRef(Message) (Game|GetPlayerCharacter 0)))
  (Variables|Default|SetPlayerPawn _player)
  (CallFunction|ShowHideWidget "NewEnumerator0" true)
  (CallFunction|InitializePlayer)
  (CallFunction|CreateShopItemCards)
  (CallFunction|AddLevelButtonUI 1))

(fn ConstructionScript)

(fn FShowWidget
  (params (Widget :type E_GameWidgets%20Enum :default "NewEnumerator0"))
  (switch Utilities|FlowControl|Switch|SwitchonE_GameWidgets Widget
    (:NewEnumerator0
      (Variables|Widgets|GetWB_Main
        (:then
          _)
        (:else
          (bind _returnvalue (UserInterface|CreateWidget "/Game/Clicker/UI/WB_Main.WB_Main_C"))
          (bind _output_get (Variables|Widgets|SetWB_Main _returnvalue))))
      (UserInterface|Viewport|AddtoViewport _output_get 0))
    (:NewEnumerator3
      (Variables|Widgets|GetWB_AscensionPopup
        (:then
          _)
        (:else
          (bind _returnvalue_2 (UserInterface|CreateWidget "/Game/Clicker/UI/WB_AscensionPopup.WB_AscensionPopup_C"))
          (bind _output_get_2 (Variables|Widgets|SetWB_AscensionPopup _returnvalue_2))))
      (UserInterface|Viewport|AddtoViewport _output_get_2 0))))

(fn FHideWidget
  (params (Widget :type E_GameWidgets%20Enum :default "NewEnumerator0"))
  (switch Utilities|FlowControl|Switch|SwitchonE_GameWidgets Widget
    (:NewEnumerator0
      (bind _wb_main (Variables|Widgets|GetWB_Main)
        (:then
          (Widget|RemovefromParent _wb_main))
        (:else)))
    (:NewEnumerator3
      (bind _wb_ascensionpopup (Variables|Widgets|GetWB_AscensionPopup)
        (:then
          (Widget|RemovefromParent _wb_ascensionpopup))
        (:else)))))

(fn FUpdateShopItemCardBuyTextColor
  (for _array_element (Variables|Default|GetShopItemCards)
    (Appearance|SetColorandOpacity (Variables|/Game/Clicker/UI/WB_ShopItemCard.WB_ShopItemCard_C|GetTXT_Buy _array_element) (Utilities|Struct|MakeSlateColor (Math|Color|SelectColor "(R=1.000000,G=0.113725,B=0.050980,A=1.000000)" "(R=0.619608,G=1.000000,B=0.050980,A=1.000000)" (> (Default|FGetItemCost (Variables|Default|GetPlayerPawn) (Variables|/Game/Clicker/UI/WB_ShopItemCard.WB_ShopItemCard_C|GetItemInfo _array_element)) (Variables|/Game/Clicker/Blueprints/Player/BP_Player.BP_Player_C|GetAmountOfCoins (Variables|Default|GetPlayerPawn))))) :!class /Script/UMG.TextBlock)
    (Widget|SetIsEnabled (Variables|/Game/Clicker/UI/WB_ShopItemCard.WB_ShopItemCard_C|GetBTN_Buy _array_element) (select (> (Default|FGetItemCost (Variables|Default|GetPlayerPawn) (Variables|/Game/Clicker/UI/WB_ShopItemCard.WB_ShopItemCard_C|GetItemInfo _array_element)) (Variables|/Game/Clicker/Blueprints/Player/BP_Player.BP_Player_C|GetAmountOfCoins (Variables|Default|GetPlayerPawn))) false true))))

(fn GetPlayerControllerRef
  (return self))