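; Player Blueprint for a clicker game that owns the coin balance, bought items, cursor damage and total DPS.
; Purchases deduct a count-based cost, spawn the item and update the shop UI, then raise cursor damage or recompute DPS with ascension multipliers and check ascension criteria.
; A looping timer damages the spawned enemy with DPS scaled to its interval.
; Enhanced Input clicks only swap the cursor widget image.
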(event Custom|AutoDamage
  ;[0.1412 0.2667 0.8431 0.3608] Applies Autodamage
  (bind _returnvalue (Utilities|Time|SetTimerbyFunctionName 0 "f_AutoDamage" (Variables|Damage|GetAutoDamageTimerTime) true))
  (Variables|Damage|SetAutoDamageHandle _returnvalue))

(event Custom|UpdateAmountOfCoins
  (params (AmountOfCoins :type Integer) (bAdd :type Boolean))
  ;[0.1412 0.2667 0.8431 0.3608] Updates the amount of coins for the player.
  (bind _output_get (Variables|Coins&Shop|SetAmountOfCoins (select bAdd (+ AmountOfCoins (Variables|Coins&Shop|GetAmountOfCoins)) (- AmountOfCoins (Variables|Coins&Shop|GetAmountOfCoins)))))
  (Default|UpdateCoinsAmountUI (Variables|/Game/Clicker/Blueprints/PC_Clicker.PC_Clicker_C|GetWB_Main (Variables|References|GetPlayerController)) _output_get))

(event Custom|PurchaseItem
  (params (Item :type ST%20Item%20Info%20Structure) (ShopItemCard :type WB%20Shop%20Item%20Card%20Object%20Reference))
  (bind (_name _item _dps) (Utilities|Struct|BreakST_ItemInfo Item))
  (bind _itemsbought (Variables|Coins&Shop|GetItemsBought))
  (bind _playercontroller (Variables|References|GetPlayerController))
  (bind _value (Utilities|Map|Find _itemsbought _name))
  ;[0.1412 0.2667 0.8431 0.3608] Purchases the item from the item shop
  (Audio|PlaySound2D (Variables|SFX|GetPurchaseSFX) 1.0 1.0 0.0 0 0)
  (bind _output_get (Variables|Coins&Shop|SetAmountOfCoins (- (Variables|Coins&Shop|GetAmountOfCoins) (CallFunction|FGetItemCost Item))))
  (Default|UpdateCoinsAmountUI (Variables|/Game/Clicker/Blueprints/PC_Clicker.PC_Clicker_C|GetWB_Main (Variables|References|GetPlayerController)) _output_get)
  (Utilities|Map|Add (Variables|Coins&Shop|GetItemsBought) _name (+ _value 1))
  (Default|UpdateItemsBoughtUI ShopItemCard)
  (Default|UpdateItemCost ShopItemCard)
  (Default|FUpdateShopItemCardBuyTextColor _playercontroller)
  (Default|SpawnItem _playercontroller (Utilities|Struct|BreakST_ItemInfo Item) (Utilities|Array|Get(acopy) (Default|FGetItemSpawnPoints (Variables|References|GetGameMode) _item) (- _value 1)))
  (if (Utilities|Enum|Equal(Enum) _item "NewEnumerator10")
    (CallFunction|FIncreaseCursorDamage (* (Utilities|Struct|BreakST_Ascension (CallFunction|FGetAscensionDamageMultiplier (Variables|/Game/Clicker/Blueprints/GM_Clicker.GM_Clicker_C|GetAscensionLevel (Variables|References|GetGameMode)))) _dps))
    (else
      (CallFunction|FUpdateTotalDPS)))
  (Default|UpdateTooltipUI (Variables|/Game/Clicker/Blueprints/PC_Clicker.PC_Clicker_C|GetWB_ShopTooltip (Variables|References|GetPlayerController)) Item)
  (Default|FCheckAscensionCriteriaMet (Variables|References|GetGameMode)))

(event Input|EnhancedActionEvents|EnhancedInputActionIA_MouseClick
  (params (ActionValue :type Boolean) (ElapsedSeconds :type Float%20%28double-precision%29) (TriggeredSeconds :type Float%20%28double-precision%29) (InputAction :type Input%20Action%20Object%20Reference :default "/Game/Clicker/Blueprints/Player/Input/IA_MouseClick.IA_MouseClick"))
  (bind _playercontroller (Variables|References|GetPlayerController))
  (bind _wb_mousecursor (Variables|/Game/Clicker/Blueprints/PC_Clicker.PC_Clicker_C|GetWB_MouseCursor _playercontroller))
  ;[0.1412 0.2667 0.8431 0.3608] Updates the Mouse Cursor Widget state
  (:Triggered
    (Default|SetMouseCursorImage _wb_mousecursor "NewEnumerator1"))
  (:Completed
    (Default|SetMouseCursorImage _wb_mousecursor "NewEnumerator0")))

(event EventBeginPlay
  ;[0.1412 0.2667 0.8431 0.3608] Begin Play - References, Updates the UI and starts AutoDamage
  (bind _playercontroller (Class|BPIPlayerController|GetPlayerControllerRef(Message) (Game|GetPlayerController 0)))
  (Variables|References|SetPlayerController _playercontroller)
  (bind _gamemode (Class|BPIGameMode|GetGameModeRef(Message) (Game|GetGameMode)))
  (Variables|References|SetGameMode _gamemode)
  (Utilities|IsValid (PlayerController|LocalPlayerSubsystems|GetEnhancedInputLocalPlayerSubsystem (Variables|References|GetPlayerController))
    (:Is%20Valid
      (Input|AddMappingContext (PlayerController|LocalPlayerSubsystems|GetEnhancedInputLocalPlayerSubsystem (Variables|References|GetPlayerController)) "/Game/Clicker/Blueprints/Player/Input/IMC_Default.IMC_Default" 0 "(bIgnoreAllPressedKeysUntilRelease=True,bForceImmediately=False,bNotifyUserSettings=False)")
      (Default|UpdateCoinsAmountUI (Variables|/Game/Clicker/Blueprints/PC_Clicker.PC_Clicker_C|GetWB_Main (Variables|References|GetPlayerController)) (Variables|Coins&Shop|GetAmountOfCoins))
      (CallFunction|AutoDamage))))

(fn ConstructionScript)

(fn FDoesPlayerHaveEnoughCoins
  (params (ItemCost :type Integer))
  (return (>= (Variables|Coins&Shop|GetAmountOfCoins) ItemCost)))

(fn FGetItemCost
  (params (Item :type ST%20Item%20Info%20Structure))
  (bind (_name _thumbnail _item) (Utilities|Struct|BreakST_ItemInfo Item))
  (bind _itemsbought (Variables|Coins&Shop|GetItemsBought))
  (bind _value (Utilities|Map|Find _itemsbought _name))
  (bind _itemcostinfo (CallFunction|FGetItemCost _value))
  (bind (_mouseclick _lightfeathercost _torch _runeoftime _theprotector _knighthelmet _kingscrown _orcskull _grandwizardhat _luckyrainbow _crownofevil) (Utilities|Struct|BreakST_ItemCost _itemcostinfo))
  (return (Utilities|Select :Index _item :NewEnumerator10 _mouseclick :NewEnumerator0 _lightfeathercost :NewEnumerator1 _torch :NewEnumerator2 _runeoftime :NewEnumerator3 _theprotector :NewEnumerator4 _knighthelmet :NewEnumerator5 _kingscrown :NewEnumerator6 _orcskull :NewEnumerator7 _grandwizardhat :NewEnumerator8 _luckyrainbow :NewEnumerator9 _crownofevil)))

(fn FAutoDamage
  (Game|Damage|ApplyDamage (Variables|/Game/Clicker/Blueprints/PC_Clicker.PC_Clicker_C|GetSpawnedEnemy (Variables|References|GetPlayerController)) (/ (Variables|Damage|GetTotalDPS) (/ 1.0 (Variables|Damage|GetAutoDamageTimerTime))) 0 0 "/Game/Clicker/Blueprints/BP_AutoDamage.BP_AutoDamage_C"))

(fn FUpdateTotalDPS
  (bind _keys (Utilities|Map|Keys (Variables|Coins&Shop|GetItemsBought)))
  (for (_array_element _array_index) _keys
    (if (Utilities|Enum|NotEqual(Enum) (.Item (Utilities|Struct|BreakST_ItemInfo (CallFunction|FGetItemInfo _array_element))) "NewEnumerator10")
      (bind _values (Utilities|Map|Values (Variables|Coins&Shop|GetItemsBought)))
      (LocalVariables|SetLocalTotalDPS (+ (LocalVariables|GetLocalTotalDPS) (* (Utilities|Array|Get(acopy) _values _array_index) (* (.DPS (Utilities|Struct|BreakST_ItemInfo (CallFunction|FGetItemInfo _array_element))) (Utilities|Struct|BreakST_Ascension (CallFunction|FGetAscensionDamageMultiplier (Variables|/Game/Clicker/Blueprints/GM_Clicker.GM_Clicker_C|GetAscensionLevel (Variables|References|GetGameMode))))))))))
  (Variables|Damage|SetTotalDPS (LocalVariables|GetLocalTotalDPS)))

(fn FIncreaseCursorDamage
  (params (DamageToAdd :type Float%20%28double-precision%29))
  (Variables|Damage|SetCursorDamage (+ (Variables|Damage|GetCursorDamage) DamageToAdd)))

(fn GetPlayerRef
  (return self))