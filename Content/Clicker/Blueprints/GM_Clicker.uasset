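; Game mode for a clicker game, managing level progression, enemy spawning, the round timer and ascension.
; Level and enemy lookups choose the enemy the player controller spawns, while a looping timer restores its health whenever time runs out.
; Owning every shop item reveals the ascension overlay, and restarting raises AscensionLevel while resetting progress.
; It also serves per-item spawn point arrays, though their grid-filling logic is disconnected from its loop.
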(event Custom|UnlockLevel
  (if (== (Variables|Default|GetCurrentLevel) (Variables|Default|GetUnlockedLevel))
    (bind _result (Math|Integer|IncrementInt (Variables|Default|GetUnlockedLevel))
      (:%20%20
        (if (<= _result (Variables|Default|GetMaxLevel))
          (Default|AddLevelButtonUI (Variables|Default|GetPlayerController) (Variables|Default|GetUnlockedLevel))
          (Audio|PlaySound2D (Utilities|Select :Index (.EnemyType (Utilities|Struct|BreakST_EnemyInfo (CallFunction|FGetEnemyInfo (Utilities|Struct|BreakST_LevelInfo (CallFunction|FGetLevelInfo (Variables|Default|GetUnlockedLevel)))))) :NewEnumerator5 (Variables|Default|GetLevelUnlockedSFXNormal) :NewEnumerator6 (Variables|Default|GetLevelUnlockedSFXBoss)) 1.0 1.0 0.0 0 0))))))

(event Custom|SetCurrentLevel
  (params (Level :type Integer))
  (bind (_enemy _spawntransform) (CallFunction|FGetEnemytoSpawnforCurrentLevel))
  (Variables|Default|SetCurrentLevel Level)
  (bind _spawnedenemy (Variables|/Game/Clicker/Blueprints/PC_Clicker.PC_Clicker_C|GetSpawnedEnemy (Variables|Default|GetPlayerController))
    (:then
      (Actor|DestroyActor _spawnedenemy))
    (:else
      _))
  (Default|SpawnEnemy (Variables|Default|GetPlayerController) _enemy _spawntransform))

(event Custom|StartRoundTimer
  (Variables|Default|SetCurrentRoundTimer (Variables|Default|GetInitialRoundTimer))
  (bind _returnvalue (Utilities|Time|SetTimerbyEvent (delegate Custom|RoundTimerLoop) (Variables|Default|GetRoundTimerTime) true))
  (Variables|Default|SetRoundTimerHandle _returnvalue))

(event Custom|RoundTimerLoop
  (bind _output_get (Variables|Default|SetCurrentRoundTimer (Math|Float|Clamp(Float) (- (Variables|Default|GetCurrentRoundTimer) (Variables|Default|GetRoundTimerTime)) 0.0 (Variables|Default|GetCurrentRoundTimer))))
  (Default|UpdateTimerUI (Variables|/Game/Clicker/Blueprints/PC_Clicker.PC_Clicker_C|GetWB_Main (Variables|Default|GetPlayerController)) _output_get)
  (if (== (Variables|Default|GetCurrentRoundTimer) 0.0)
    (Default|RestoreHealth (Variables|/Game/Clicker/Blueprints/PC_Clicker.PC_Clicker_C|GetSpawnedEnemy (Variables|Default|GetPlayerController)))
    (Variables|Default|SetCurrentRoundTimer (Variables|Default|GetInitialRoundTimer))))

(event EventBeginPlay
  (bind (_enemy _spawntransform) (CallFunction|FGetEnemytoSpawnforCurrentLevel))
  (bind _returnvalue (Actor|GetActorOfClass "/Game/Clicker/Blueprints/SpawnPoints/BP_EnemySpawnPoint.BP_EnemySpawnPoint_C"))
  (Variables|Default|SetEnemySpawnPoint _returnvalue)
  (bind _playercontroller (Class|BPIPlayerController|GetPlayerControllerRef(Message) (Game|GetPlayerController 0)))
  (bind _output_get (Variables|Default|SetPlayerController _playercontroller))
  (bind _player (Class|BPIPlayer|GetPlayerRef(Message) (Game|GetPlayerCharacter 0)))
  (Variables|Default|SetPlayerPawn _player)
  (CallFunction|FSetItemSpawnPoints)
  (bind _outrownames (DataTable|GetDataTableRowNames "/Game/Clicker/Blueprints/DataTables/DT_ItemInfo.DT_ItemInfo"))
  (Variables|Default|SetAmountOfShopItems (Utilities|Array|Length _outrownames))
  (Default|SpawnEnemy _output_get _enemy _spawntransform)
  (CallFunction|StartRoundTimer))

(fn ConstructionScript)

(fn FGetEnemytoSpawnforCurrentLevel
  (return (.Class (Utilities|Struct|BreakST_EnemyInfo (CallFunction|FGetEnemyInfo (Utilities|Struct|BreakST_LevelInfo (CallFunction|FGetLevelInfo (Variables|Default|GetCurrentLevel)))))) (Transformation|GetActorTransform (Variables|Default|GetEnemySpawnPoint))))

(fn FSetItemSpawnPoints
  (bind _outactors (Actor|GetAllActorsOfClass "/Game/Clicker/Blueprints/SpawnPoints/BP_ItemSpawnPoint.BP_ItemSpawnPoint_C"))
  (bind _output_get (LocalVariables|SetLocalItemSpawnPoints _outactors))
  (if (> (Utilities|Array|Length _output_get) 0)
    (for _index (range 0 (LocalVariables|GetLocalLoopLastIndex))
      _)))

(fn FGetItemSpawnPoints
  (params (ItemName :type E_Items%20Enum :default "NewEnumerator10"))
  (switch Utilities|FlowControl|Switch|SwitchonE_Items ItemName
    (:NewEnumerator10
      (return (Variables|ItemSpawnPoints|GetMouseClickSpawnPoints)))
    (:NewEnumerator0
      (return (Variables|ItemSpawnPoints|GetLightFeatherSpawnPoints)))
    (:NewEnumerator1
      (return (Variables|ItemSpawnPoints|GetTorchSpawnPoints)))
    (:NewEnumerator2
      (return (Variables|ItemSpawnPoints|GetRuneOfTimeSpawnPoints)))
    (:NewEnumerator3
      (return (Variables|ItemSpawnPoints|GetTheProtectorSpawnPoints)))
    (:NewEnumerator4
      (return (Variables|ItemSpawnPoints|GetKnightHelmetSpawnPoints)))
    (:NewEnumerator5
      (return (Variables|ItemSpawnPoints|GetKingsCrownSpawnPoints)))
    (:NewEnumerator6
      (return (Variables|ItemSpawnPoints|GetOrcSkullSpawnPoints)))
    (:NewEnumerator7
      (return (Variables|ItemSpawnPoints|GetGrandWizardHatSpawnPoints)))
    (:NewEnumerator8
      (return (Variables|ItemSpawnPoints|GetLuckyRainbowSpawnPoints)))
    (:NewEnumerator9
      (return (Variables|ItemSpawnPoints|GetCrownOfEvilSpawnPoints)))))

(fn FCheckAscensionCriteriaMet
  (if (not (Variables|Default|GetbAscensionCriteriaMet))
    (bind _keys (Utilities|Map|Keys (Variables|/Game/Clicker/Blueprints/Player/BP_Player.BP_Player_C|GetItemsBought (Variables|Default|GetPlayerPawn))))
    (if (== (Utilities|Array|Length _keys) (Variables|Default|GetAmountOfShopItems))
      (bind _values (Utilities|Map|Values (Variables|/Game/Clicker/Blueprints/Player/BP_Player.BP_Player_C|GetItemsBought (Variables|Default|GetPlayerPawn))))
      (bind _array_element (Utilities|Array|ForEachLoopwithBreak _values :!label _label)
        (:LoopBody
          (if (>= _array_element 1)
            (Math|Integer|IncrementInt (LocalVariables|GetLocalCounter))
            (else
              (goto _label Break))))
        (:Completed
          (if (== (LocalVariables|GetLocalCounter) (Variables|Default|GetAmountOfShopItems))
            (Variables|Default|SetbAscensionCriteriaMet true)
            (Widget|SetVisibility (Variables|/Game/Clicker/UI/WB_Main.WB_Main_C|GetOV_Ascension (Variables|/Game/Clicker/Blueprints/PC_Clicker.PC_Clicker_C|GetWB_Main (Variables|Default|GetPlayerController))) "SelfHitTestInvisible")))))))

(fn FRestartGame
  (bind _playercontroller (Variables|Default|GetPlayerController))
  (bind _playerpawn (Variables|Default|GetPlayerPawn))
  (Math|Integer|IncrementInt (Variables|Default|GetAscensionLevel)
    (:%20%20
      (Variables|Default|SetbAscensionCriteriaMet false)
      (Variables|Default|SetUnlockedLevel 1)
      (Variables|Default|SetCurrentLevel 1)
      (Widget|Panel|ClearChildren (Variables|/Game/Clicker/UI/WB_Main.WB_Main_C|GetVB_LevelList (Variables|/Game/Clicker/Blueprints/PC_Clicker.PC_Clicker_C|GetWB_Main _playercontroller)))
      (Default|AddLevelButtonUI _playercontroller (Variables|Default|GetUnlockedLevel))
      (bind _output_get (Variables|/Game/Clicker/Blueprints/Player/BP_Player.BP_Player_C|SetAmountOfCoins (Variables|Default|GetPlayerPawn) 0))
      (Default|UpdateCoinsAmountUI (Variables|/Game/Clicker/Blueprints/PC_Clicker.PC_Clicker_C|GetWB_Main (Variables|Default|GetPlayerController)) _output_get)
      (Utilities|Map|Clear (Variables|/Game/Clicker/Blueprints/Player/BP_Player.BP_Player_C|GetItemsBought (Variables|Default|GetPlayerPawn)))
      (Default|CreateShopItemCards (Variables|Default|GetPlayerController))
      (Variables|/Game/Clicker/Blueprints/Player/BP_Player.BP_Player_C|SetTotalDPS _playerpawn 0.0)
      (Variables|/Game/Clicker/Blueprints/Player/BP_Player.BP_Player_C|SetCursorDamage _playerpawn 15.0)
      (CallFunction|SetCurrentLevel (Variables|Default|GetCurrentLevel)))))

(fn GetGameModeRef
  (return self))