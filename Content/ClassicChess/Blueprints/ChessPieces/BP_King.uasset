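; BP_King is the king piece in a chess game, providing helpers to validate and highlight its moves, including castling.
; Square checks query the game mode's occupant data, rejecting off-board and friendly-occupied squares without testing for attacks.
; Castling requires an unmoved king not in check, then scans both Y directions for empty squares ending in an unmoved rook.
; ShowPossibleMoves only returns false, and nothing here calls the highlight or castling entry points.
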(fn ConstructionScript
  (|CallParentFunction))

(fn ShowPossibleMoves
  (return false))

(fn HighlightKingSquare
  (params (XIncr :type Integer) (YIncr :type Integer))
  (LocalVariables|SetTempX (+ (Variables|Default|GetX) XIncr))
  (LocalVariables|SetTempY (+ (Variables|Default|GetY) YIncr))
  (if (GamePlay|IsValidMoveforKing (LocalVariables|GetTempX) (LocalVariables|GetTempY))
    (CallFunction|HighlightPotentialSquare (LocalVariables|GetTempX) (LocalVariables|GetTempY) (Variables|Default|GetColor))))

(fn EvaluateCastleSquares
  (Variables|Default|SetKindCanCastle false)
  (if (not (Variables|Default|GetKingHasCastled))
    (if (Variables|Default|GetIsInitialMove)
      (if (not (Default|IsActiveKingCheckStatus (Variables|Default|GetGameModeRef)))
        (Utilities|FlowControl|Sequence
          (:then_0
            (GamePlay|EvaluateCastlePath 1))
          (:then_1
            (GamePlay|EvaluateCastlePath -1)))
        (else
          (Variables|Default|SetKindCanCastle false :!label _label)))
      (else
        (goto _label)))))

(fn HighlightCastleSquares
  (params (IsPositive :type Boolean))
  (if IsPositive
    (bind _output_get (LocalVariables|SetTempY (+ (Variables|Default|GetY) 2)))
    (CallFunction|HighlightPotentialSquare (Variables|Default|GetX) _output_get (Variables|Default|GetColor))
    (Variables|Default|SetKindCanCastle true)
    (else
      (bind _output_get_2 (LocalVariables|SetTempY (+ (Variables|Default|GetY) -2)))
      (CallFunction|HighlightPotentialSquare (Variables|Default|GetX) _output_get_2 (Variables|Default|GetColor))
      (Variables|Default|SetKindCanCastle true))))

(fn IsValidMoveforKing
  (params (X :type Integer) (Y :type Integer))
  (bind _gamemoderef (Variables|Default|GetGameModeRef))
  (bind _color (Variables|Default|GetColor))
  (bind (_occupant _isoccupied _isoccupiedbyfriend _isvalidsquare) (Default|GetOccupant _gamemoderef X Y _color))
  (if _isvalidsquare
    (if _isoccupiedbyfriend
      (return false)
      (else
        (return true)))
    (else
      (return false))))

(fn EvaluateCastlePath
  (params (YInc :type Integer))
  (LocalVariables|SetIsPositive (> YInc 0))
  (LocalVariables|SetTempY (Variables|Default|GetY))
  (LocalVariables|SetCanContinue true)
  (while (LocalVariables|GetCanContinue)
    (LocalVariables|SetTempY (+ YInc (LocalVariables|GetTempY)))
    (if (and (< (LocalVariables|GetTempY) 8) (> (LocalVariables|GetTempY) 1))
      (LocalVariables|SetCanContinue (not (.IsOccupied (Default|GetOccupant (Variables|Default|GetGameModeRef) (Variables|Default|GetX) (LocalVariables|GetTempY) (Variables|Default|GetColor)))))
      (else
        (if (and (.bSuccess (Utilities|Casting|CastToBP_Rook (.Occupant (Default|GetOccupant (Variables|Default|GetGameModeRef) (Variables|Default|GetX) (LocalVariables|GetTempY) (Variables|Default|GetColor))))) (.IsOccupied (Default|GetOccupant (Variables|Default|GetGameModeRef) (Variables|Default|GetX) (LocalVariables|GetTempY) (Variables|Default|GetColor))))
          (if (Variables|/Game/ClassicChess/Blueprints/ChessPieces/BP_ChessPiece.BP_ChessPiece_C|GetIsInitialMove (.AsBP%20Rook (Utilities|Casting|CastToBP_Rook (.Occupant (Default|GetOccupant (Variables|Default|GetGameModeRef) (Variables|Default|GetX) (LocalVariables|GetTempY) (Variables|Default|GetColor))))))
            (GamePlay|HighlightCastleSquares (LocalVariables|GetIsPositive))))
        (LocalVariables|SetCanContinue false)))))